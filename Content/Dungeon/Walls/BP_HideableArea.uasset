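; BP_HideableArea is a dungeon area actor that hides and shows the BP_FadeWall actors overlapping it.
; StartHideObjects and EndHideObjects set the HideObjects flag, then both run UpdateHidingActors.
; That function queries overlapping fade walls at call time and calls Hide or Show on each according to the flag, so it keeps no list of walls.
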(event `self.ReceiveBeginPlay`
  (set `self.HideObjects?` false))

(event `StartHideObjects`
  (set `self.HideObjects?` true)
  (`self.UpdateHidingActors` :!label _label))

(event `EndHideObjects`
  (set `self.HideObjects?` false)
  (goto _label))

(fn `UpdateHidingActors`
  (for _array_element (`self.GetOverlappingActors` "/Game/Dungeon/Walls/BP_FadeWall.BP_FadeWall_C")
    (bind _asbp_fade_wall (cast `/Game/Dungeon/Walls/BP_FadeWall` _array_element))
    (if (`self.HideObjects?`)
      (`/Game/Dungeon/Walls/BP_FadeWall.Hide` _asbp_fade_wall)
      (else
        (`/Game/Dungeon/Walls/BP_FadeWall.Show` _asbp_fade_wall))))
  (return))

(fn `UserConstructionScript`)