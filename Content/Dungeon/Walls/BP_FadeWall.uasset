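; Dungeon wall actor that fades out on Hide and back in on Show.
; Tick steps the Opacity of a dynamic material on WallPreset by FadeSpeed until it reaches either limit.
; WallBottom becomes visible when hiding starts and disappears once the wall is fully restored.
; The fade material is applied during transitions, and M_dungeon_main_Inst replaces it at full opacity.
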(event `self.ReceiveBeginPlay`
  (bind _material (`self.Material`))
  (bind _wall_bottom (`self.Wall_Bottom`))
  (`SceneComponent.SetVisibility` (`self.Wall_Bottom`) false false)
  (bind _returnvalue (`KismetMaterialLibrary.CreateDynamicMaterialInstance` _material _material))
  (set `self.DynamicMaterial` _returnvalue)
  (bind _returnvalue_2 (`PrimitiveComponent.CreateDynamicMaterialInstance` _wall_bottom 0 (`PrimitiveComponent.GetMaterial` _wall_bottom 0)))
  (set `self.OriginalMaterial` _returnvalue_2))

(event `self.ReceiveTick`
  (params (DeltaSeconds :type "Float (single-precision)"))
  (bind _shouldhide (`self.ShouldHide`))
  (if _shouldhide
    (`self.SetUpMaterial` (`self.DynamicMaterial`) :!label _label)
    (`self.UpdateVisibility` (* DeltaSeconds (`self.FadeSpeed`)) _shouldhide)
    (elif (`self.ShouldShow`)
      (goto _label))))

(event `Hide`
  (`SceneComponent.SetVisibility` (`self.Wall_Bottom`) true true)
  (set `self.ShouldHide` true)
  (set `self.ShouldShow` false))

(event `Show`
  (set `self.ShouldHide` false)
  (set `self.ShouldShow` true))

(fn `ResetVisibility`
  (bind _dynamicmaterial (`self.DynamicMaterial`))
  (`MaterialInstanceDynamic.K2_GetScalarParameterValue` _dynamicmaterial "Opacity")
  (`MaterialInstanceDynamic.SetScalarParameterValue` _dynamicmaterial "Opacity" 1.0))

(fn `SetUpMaterial`
  (params (Material :type "MaterialInstance Object Reference"))
  (`PrimitiveComponent.SetMaterial` (`self.Wall_Preset`) 0 Material)
  (return))

(fn `UpdateVisibility`
  (params (Amount :type "Float (double-precision)") (ShouldHide :type Boolean))
  (bind _dynamicmaterial (`self.DynamicMaterial`))
  (bind _returnvalue (`MaterialInstanceDynamic.K2_GetScalarParameterValue` _dynamicmaterial "Opacity"))
  (if ShouldHide
    (bind _returnvalue_2 (- _returnvalue Amount))
    (`MaterialInstanceDynamic.SetScalarParameterValue` _dynamicmaterial "Opacity" _returnvalue_2)
    (set `self.ShouldHide` (not (<= _returnvalue_2 0.0)))
    (else
      (bind _returnvalue_3 (+ _returnvalue Amount))
      (`MaterialInstanceDynamic.SetScalarParameterValue` _dynamicmaterial "Opacity" _returnvalue_3)
      (bind _returnvalue_4 (>= _returnvalue_3 1.0))
      (set `self.ShouldShow` (not _returnvalue_4))
      (if _returnvalue_4
        (`self.SetUpMaterial` "/Game/Dungeon/Materials/M_dungeon_main_Inst.M_dungeon_main_Inst")
        (`SceneComponent.SetVisibility` (`self.Wall_Bottom`) false true)))))

(fn `UserConstructionScript`)