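; Player controller for an RPG Default_Character, combining click-to-move with camera-relative axis movement.
; While left click is held, a Tick-fed gate repeatedly moves the pawn toward the cursor hit; release spawns a goal decal there.
; Axis movement cancels that command via CancelMovementCommand, stopping the character and destroying the decal.
; Holding EnableTurning lets Turn and LookUp rotate the camera arm, with pitch clamped.
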(event `self.ReceiveBeginPlay`
  ;[1 1 1] On start setting controlledCharacter
  (bind _asdefault_character (cast `/Game/RPG/Characters/Default_Character` (`self.K2_GetPawn`)))
  (set `self.ControlledCharacter` _asdefault_character))

(event `InputAction|EnableTurning`
  (params (Key :type "Key Structure" :default "AnyKey"))
  ;[1 1 1] Right mouse button
  (:`Pressed`
    (set `self.CanTurn?` true))
  (:`Released`
    (set `self.CanTurn?` false)))

(event `InputAxis|LookUp`
  (params (AxisValue :type "Float (single-precision)"))
  (bind _cameraarm (`/Game/RPG/Characters/Default_Character.CameraArm` (`self.ControlledCharacter`)))
  ;[1 1 1] LookUp Event
  (if (and (!= AxisValue 0.0) (`self.CanTurn?`))
    (`SceneComponent.K2_SetRelativeRotation` _cameraarm (`KismetMathLibrary.MakeRotator` (.roll (.rotation (`SceneComponent.GetRelativeTransform` _cameraarm))) (`KismetMathLibrary.FClamp` (+ (.pitch (.rotation (`SceneComponent.GetRelativeTransform` _cameraarm))) (* AxisValue 1.5)) -60.0 -20.0) (.yaw (.rotation (`SceneComponent.GetRelativeTransform` _cameraarm)))) false false)))

(event `InputAxis|Turn`
  (params (AxisValue :type "Float (single-precision)"))
  (bind _cameraarm (`/Game/RPG/Characters/Default_Character.CameraArm` (`self.ControlledCharacter`)))
  ;[1 1 1] Axis Turn Event
  (if (and (!= AxisValue 0.0) (`self.CanTurn?`))
    (`SceneComponent.K2_SetRelativeRotation` _cameraarm (`KismetMathLibrary.MakeRotator` (.roll (.rotation (`SceneComponent.GetRelativeTransform` _cameraarm))) (.pitch (.rotation (`SceneComponent.GetRelativeTransform` _cameraarm))) (+ (.yaw (.rotation (`SceneComponent.GetRelativeTransform` _cameraarm))) (* AxisValue 2.0))) false false)))

(event `self.ReceiveTick`
  (params (DeltaSeconds :type "Float (single-precision)"))
  ;[1 1 1] Mouse movement and decal spawning
  (`/Engine/EditorBlueprintResources/StandardMacros.Gate` true :!label _label
    (:`Exit`
      (`self.CancelMovementCommand`)
      (`NavigationSystem.SimpleMoveToLocation` self (`.Location` (`GameplayStatics.BreakHitResult` (`self.GetHitResultUnderCursorByChannel` "TraceTypeQuery1")))))))

(event `InputAction|LeftClick`
  (params (Key :type "Key Structure" :default "AnyKey"))
  ;[1 1 1] Mouse movement and decal spawning
  (:`Pressed`
    (goto _label :!via `Open`))
  (:`Released`
    (bind _returnvalue (`|SpawnActorFromClass` "/Game/RPG/Blueprints/BP_GoalDecal.BP_GoalDecal_C" (`KismetMathLibrary.MakeTransform` (`.Location` (`GameplayStatics.BreakHitResult` (`self.GetHitResultUnderCursorByChannel` "TraceTypeQuery1")))) "Undefined" "OverrideRootScale" null self))
    (set `self.Current_GoalDecal` _returnvalue)
    (set `self.HasMouseMovementCommand?` true)
    (goto _label :!via `Close`)))

(event `InputAxis|MoveForward`
  (params (AxisValue :type "Float (single-precision)"))
  (bind _controlledcharacter (`self.ControlledCharacter`))
  ;[1 1 1] Moving forward and backward
  (if (!= AxisValue 0.0)
    (if (`self.HasMouseMovementCommand?`)
      (`self.CancelMovementCommand`))
    (`Pawn.AddMovementInput` _controlledcharacter (`KismetMathLibrary.GetForwardVector` (`KismetMathLibrary.MakeRotator` 0.0 0.0 (.yaw (.rotation (`SceneComponent.GetRelativeTransform` (`/Game/RPG/Characters/Default_Character.CameraArm` _controlledcharacter)))))) AxisValue false)))

(event `InputAxis|MoveRight`
  (params (AxisValue :type "Float (single-precision)"))
  (bind _controlledcharacter (`self.ControlledCharacter`))
  ;[1 1 1] Moving right and left
  (if (!= AxisValue 0.0)
    (if (`self.HasMouseMovementCommand?`)
      (`self.CancelMovementCommand`))
    (`Pawn.AddMovementInput` _controlledcharacter (`KismetMathLibrary.GetRightVector` (`KismetMathLibrary.MakeRotator` 0.0 0.0 (.yaw (.rotation (`SceneComponent.GetRelativeTransform` (`/Game/RPG/Characters/Default_Character.CameraArm` _controlledcharacter)))))) AxisValue false)))

(fn `CancelMovementCommand`
  (`/Engine/EditorBlueprintResources/StandardMacros.IsValid` (`self.Current_GoalDecal`)
    (:`Is Valid`
      (`MovementComponent.StopMovementImmediately` (`Character.CharacterMovement` (`self.ControlledCharacter`)))
      (`self.K2_DestroyActor` (`self.Current_GoalDecal`))
      (set `self.HasMouseMovementCommand?` false)
      (set `self.Current_GoalDecal` null))
    (:`Is Not Valid`
      _))
  (return))

(fn `UserConstructionScript`)