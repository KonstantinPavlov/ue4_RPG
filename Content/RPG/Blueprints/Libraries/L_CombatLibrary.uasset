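; Combat function library for an RPG with helpers for identifying enemies and resolving hit damage.
; IsEnemy treats any actor whose class is or derives from BP_Behavior_AI as an enemy.
; CalculateFinalDamage applies random variance to base damage, rolls a percentage critical chance, scales crits by a multiplier chosen per damage type, and returns the rounded damage with a critical flag.
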(fn `CalculateFinalDamage`
  (params (BaseDamage :type "Float (double-precision)") (CritChance :type Integer) (DamageType :type "/Game/RPG/Blueprints/Enums/E_DamageTypes Enum"))
  (returns (FinalDamage :type Integer) (`Critical?` :type Boolean))
  (locals (CurrentDamage :type "Float (double-precision)") (LocalCrit :type Boolean))
  (set `local.CurrentDamage` (* BaseDamage (`KismetMathLibrary.RandomFloatInRange` 0.8 1.1)))
  (bind _output_get (set `local.LocalCrit` (<= (`KismetMathLibrary.RandomIntegerInRange` 1 100) CritChance)))
  (if _output_get
    (set `local.CurrentDamage` (* (`local.CurrentDamage`) (select `/Game/RPG/Blueprints/Enums/E_DamageTypes` DamageType :`NewEnumerator0` 1.5 :`NewEnumerator1` 1.75 :`NewEnumerator2` 2.0 :!type "Float (single-precision)"))))
  (return (`KismetMathLibrary.Round` (`local.CurrentDamage`)) (`local.LocalCrit`)))

(fn `IsEnemy?`
  (params (Actor :type "Actor Object Reference"))
  (returns (Out :type Boolean))
  (bind _returnvalue (`GameplayStatics.GetObjectClass` Actor))
  (return (or (== _returnvalue "/Game/RPG/Characters/AI/Behavior_AI/BP_Behavior_AI.BP_Behavior_AI_C") (`KismetMathLibrary.ClassIsChildOf` _returnvalue "/Game/RPG/Characters/AI/Behavior_AI/BP_Behavior_AI.BP_Behavior_AI_C"))))