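; BP_MagicProjectile is a homing magic missile that damages its assigned AI target.
; On BeginPlay it applies its speed and missile particle effect, then homes on the target's HitArrow component.
; On sphere hit it spawns an impact effect and destroys itself, applying damage with crit chance only if the hit actor is that target.
; The attacker is always reported as player pawn 0.
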(event `self.ReceiveBeginPlay`
  (bind _projectilemovement (`self.ProjectileMovement`))
  (bind _output_get (set `ProjectileMovementComponent.InitialSpeed` (`self.InitialSpeed`) _projectilemovement))
  (set `ProjectileMovementComponent.MaxSpeed` _output_get _projectilemovement)
  (`ParticleSystemComponent.SetTemplate` (`self.ParticleSystem`) (`self.MissileEffect`))
  (set `ProjectileMovementComponent.HomingTargetComponent` (`/Game/RPG/Characters/AI/Behavior_AI/BP_Behavior_AI.HitArrow` (`self.Target`)) (`self.ProjectileMovement`)))

(event `self.Sphere.OnComponentHit`
  (params (HitComponent :type "PrimitiveComponent Object Reference") (OtherActor :type "Actor Object Reference") (OtherComp :type "PrimitiveComponent Object Reference") (NormalImpulse :type "Vector Structure") (Hit :type "HitResult Structure (by ref)"))
  (`GameplayStatics.SpawnEmitterAtLocation` (`self.ImpactEffect`) (`self.K2_GetActorLocation`))
  (bind _asbp_behavior_ai (cast `/Game/RPG/Characters/AI/Behavior_AI/BP_Behavior_AI` OtherActor)
    (:`then`
      (if (== _asbp_behavior_ai (`self.Target`))
        (`/Game/RPG/Blueprints/Interfaces/I_Damageable.OnRecieveDamage` (`self.Target`) (`self.BaseDamage`) (`self.DamageType`) (`self.CritChance`) (`GameplayStatics.GetPlayerPawn` 0))))
    (:`CastFailed`
      _))
  (`self.K2_DestroyActor`))

(fn `UserConstructionScript`)