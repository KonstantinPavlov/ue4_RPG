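; Enemy AI character that patrols, attacks and takes damage, with hover health UI for the player.
; BeginPlay runs its behavior tree and seeds the blackboard; pawn sensing or incoming damage marks the player as target.
; Attacks play random montages, with a notify-driven line trace dealing damage through I_Damageable.
; OnDeath grants experience and delays destruction, but damage never reaches it because clamped Health always passes the >= 0 check.
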(event `self.ReceiveBeginPlay`
  (bind _returnvalue (`AIBlueprintHelperLibrary.GetBlackboard` self))
  ;[0.6962 0.3326 1] Begin Play Setting up Blackboard variables
  (set `self.Health` (`self.MaxHealth`))
  (`AIController.RunBehaviorTree` (`AIBlueprintHelperLibrary.GetAIController` self) (`self.BehaviorTree`))
  (`BlackboardComponent.SetValueAsVector` _returnvalue "OriginalLocation" (`self.K2_GetActorLocation`))
  (`BlackboardComponent.SetValueAsFloat` _returnvalue "PatrolRadius" (`self.PatrolRadius`))
  (`BlackboardComponent.SetValueAsFloat` _returnvalue "AttackRange" (`self.AttackRange`)))

(event `self.PawnSensing.OnSeePawn`
  (params (Pawn :type "Pawn Object Reference"))
  (bind _returnvalue (`AIBlueprintHelperLibrary.GetBlackboard` self))
  ;[1 1 1] On seen Pawn
  (if (and (== Pawn (`GameplayStatics.GetPlayerPawn` 0)) (not (`self.HasSeenPlayer?`)))
    (bind _output_get (set `self.HasSeenPlayer?` true))
    (`BlackboardComponent.SetValueAsBool` _returnvalue "HasSeenPlayer?" _output_get)
    (`BlackboardComponent.SetValueAsObject` _returnvalue "Player" Pawn)
    (set `CharacterMovementComponent.MaxWalkSpeed` (`self.MaxWalkSpeed`) (`self.CharacterMovement`))))

(event `BeginAttack`
  (params (AttackTask :type "/Game/RPG/Characters/AI/Behavior_AI/BTask_BeginAttack Object Reference"))
  (bind (_montage _sequence) (`self.GetRandomMontage`))
  ;[1 0.3822 0.442] Begin Attack
  (`self.K2_SetActorRotation` (`KismetMathLibrary.FindLookAtRotation` (`self.K2_GetActorLocation`) (`self.K2_GetActorLocation` (`GameplayStatics.GetPlayerCharacter` 0))) true)
  (`self.PlayAnimMontage` _montage)
  (`KismetSystemLibrary.Delay` _sequence)
  (`/Game/RPG/Characters/AI/Behavior_AI/BTask_BeginAttack.BeginAttackLaunched` AttackTask))

(event `AttackNotify`
  (bind _returnvalue (`self.K2_GetActorLocation`))
  ;[0.9201 1 0.2258] Attack Notify
  (bind _outhit (`KismetSystemLibrary.LineTraceSingleForObjects` :`Start` _returnvalue :`End` (+ _returnvalue (* (`self.GetActorForwardVector`) (`self.AttackDistance`))) :`ObjectTypes` (`|MakeArray` "ObjectTypeQuery3" :!type "EObjectTypeQuery Enum") :`bTraceComplex` true :`DrawDebugType` "ForDuration"))
  (bind (_bblockinghit _binitialoverlap _time _location _impactpoint _normal _impactnormal _physmat _hitactor) (`GameplayStatics.BreakHitResult` _outhit))
  (if (`KismetSystemLibrary.DoesImplementInterface` _hitactor "/Game/RPG/Blueprints/Interfaces/I_Damageable.I_Damageable_C")
    (message `/Game/RPG/Blueprints/Interfaces/I_Damageable.OnRecieveDamage` _hitactor (`self.BaseDamage`) (`self.DamageType`) (`self.CritChance`) self)))

(event `OnDeath`
  ;[1 0 0.4516] On Death Event
  (bind _returnvalue (`self.GetCurrentMontage`))
  (`/Engine/EditorBlueprintResources/StandardMacros.IsValid` _returnvalue
    (:`Is Valid`
      (`self.StopAnimMontage` _returnvalue))
    (:`Is Not Valid`
      _))
  (bind _output_get (set `self.isDead?` true))
  (`BlackboardComponent.SetValueAsBool` (`AIBlueprintHelperLibrary.GetBlackboard` null) "isDead?" _output_get)
  (`PrimitiveComponent.SetCollisionEnabled` (`self.CapsuleComponent`) "NoCollision")
  (bind _asdefault_character (cast `/Game/RPG/Characters/Character/Default_Character` (`GameplayStatics.GetPlayerCharacter` 0)))
  (`/Game/RPG/Characters/Character/Default_Character.ModifyStat` _asdefault_character "NewEnumerator3" (`self.ExpForKill`) true)
  (`KismetSystemLibrary.Delay` 60.0)
  (`self.K2_DestroyActor`))

(event `self.CursorSphere.OnBeginCursorOver`
  (params (TouchedComponent :type "PrimitiveComponent Object Reference"))
  (bind _asdefault_character (cast `/Game/RPG/Characters/Character/Default_Character` (`GameplayStatics.GetPlayerCharacter` 0)))
  (bind _mainwidget (`/Game/RPG/Characters/Character/Default_Character.GetMainWidget` _asdefault_character))
  (set `self.EnemyWidget` (`/Game/RPG/UI/Widgets/W_Main.W_EnemyHealth` _mainwidget))
  (if (not (`self.isDead?`))
    (`self.OnHovered`)
    (`self.SetEnemyWigetVisible`)
    (`self.InitWidgetText`)
    (`self.UpdateHealthBar`)
    (`PrimitiveComponent.SetRenderCustomDepth` (`self.Mesh`) true)))

(event `/Game/RPG/Blueprints/Interfaces/I_Damageable.OnRecieveDamage`
  (params (BaseDamage :type "Float (single-precision)") (DamageType :type "/Game/RPG/Blueprints/Enums/E_DamageTypes Enum" :default "NewEnumerator0") (CritChance :type Integer) (Atacker :type "Actor Object Reference"))
  (bind _returnvalue (`AIBlueprintHelperLibrary.GetBlackboard` self))
  ;[1 0.573 0.4931] On Recieve Damage
  (if (and (not (`self.isDead?`)) (not (`/Game/RPG/Blueprints/Libraries/L_CombatLibrary.IsEnemy?` Atacker)))
    (bind _finaldamage (`/Game/RPG/Blueprints/Libraries/L_CombatLibrary.CalculateFinalDamage` BaseDamage CritChance DamageType))
    (set `self.Health` (`KismetMathLibrary.Clamp` (- (`self.Health`) _finaldamage) 0 (`self.MaxHealth`)))
    (`self.UpdateHealthBar`)
    (if (>= (`self.Health`) 0)
      (`BlackboardComponent.SetValueAsObject` _returnvalue "Player" (`GameplayStatics.GetPlayerCharacter` 0))
      (bind _output_get (set `self.HasSeenPlayer?` true))
      (`BlackboardComponent.SetValueAsBool` _returnvalue "HasSeenPlayer?" _output_get)
      (else
        (`self.OnDeath`)))))

(event `self.CursorSphere.OnEndCursorOver`
  (params (TouchedComponent :type "PrimitiveComponent Object Reference"))
  (`self.OnUnHovered`)
  (`self.SetEnemyWigetNotVisible`)
  (`PrimitiveComponent.SetRenderCustomDepth` (`self.Mesh`) false))

(fn `EnemyWidgetIsVisible?`
  (returns (Out :type Boolean))
  (return (select `ESlateVisibility` (`Widget.GetVisibility` (`self.EnemyWidget`)) :`Visible` true)))

(fn `GetRandomMontage`
  (returns (Montage :type "AnimMontage Object Reference") (Sequence :type "Float (double-precision)"))
  (bind _attackmontagearray (`self.AttackMontageArray`))
  (bind _output (`|GetArrayItem` _attackmontagearray (`KismetMathLibrary.RandomIntegerInRange` 0 (- (`KismetArrayLibrary.Array_Length` _attackmontagearray) 1))))
  (return _output (`AnimSequenceBase.SequenceLength` _output)))

(fn `InitWidgetText`
  (`TextBlock.SetText` (`/Game/RPG/UI/Widgets/W_EnemyHealth.EnemyName` (`self.EnemyWidget`)) (`self.Name`)))

(fn `OnHovered`
  (set `PlayerController.CurrentMouseCursor` "Crosshairs" (`GameplayStatics.GetPlayerController` 0))
  (return))

(fn `OnUnHovered`
  (set `PlayerController.CurrentMouseCursor` "Default" (`GameplayStatics.GetPlayerController` 0))
  (return))

(fn `SetEnemyWigetNotVisible`
  (`Widget.SetVisibility` (`self.EnemyWidget`) "Hidden")
  (return))

(fn `SetEnemyWigetVisible`
  (`Widget.SetVisibility` (`self.EnemyWidget`) "Visible")
  (return))

(fn `UpdateHealthBar`
  (`ProgressBar.SetPercent` (`/Game/RPG/UI/Widgets/W_EnemyHealth.HealthBar` (`self.EnemyWidget`)) (/ (`KismetMathLibrary.Conv_IntToDouble` (`self.Health`)) (`KismetMathLibrary.Conv_IntToDouble` (`self.MaxHealth`)))))

(fn `UserConstructionScript`)